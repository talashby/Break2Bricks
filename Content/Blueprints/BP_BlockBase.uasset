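; BP_BlockBase is the base Blueprint for a block in a grid, providing animations that drop it down or slide it to connect columns.
; Two events move the root component by a step count times the owning grid's spacing, along negative X for drops and negative Y for column joins.
; Latent MoveComponentTo eases each move over a time derived from distance and DropDownSpeed, with a boolean flag set while it runs.
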(event EventAnimDropDown
  (params (iSteps :type Integer))
  (bind _returnvalue (Transformation|GetActorLocation))
  (bind (_x _y _z) (Math|Vector|BreakVector _returnvalue))
  ;[1 1 1] Drop down animation
  (Variables|Default|SetSteps iSteps)
  (Variables|Default|SetbAnimDropDown true)
  (Components|MoveComponentTo (VehicleSound|GetRootComponent) (Math|Vector|MakeVector (- _x (* (Variables|Default|GetSteps) (Variables|/Script/Break2Bricks.Break2BricksBlockGrid|GetBlockSpacing (Variables|Default|GetOwningGrid)))) _y _z) "0, 0, 0" false true (/ (* (Variables|Default|GetSteps) (Variables|/Script/Break2Bricks.Break2BricksBlockGrid|GetBlockSpacing (Variables|Default|GetOwningGrid))) (Variables|Default|GetDropDownSpeed)) false)
  (Variables|Default|SetbAnimDropDown false))

(event EventAnimConnectColumns
  (params (iSteps :type Integer))
  (bind _returnvalue (Transformation|GetActorLocation))
  (bind (_x _y _z) (Math|Vector|BreakVector _returnvalue))
  (Variables|Default|SetSteps iSteps)
  (Variables|Default|SetbAnimConnectColumns true)
  (Components|MoveComponentTo (VehicleSound|GetRootComponent) (Math|Vector|MakeVector _x (- _y (* (Variables|Default|GetSteps) (Variables|/Script/Break2Bricks.Break2BricksBlockGrid|GetBlockSpacing (Variables|Default|GetOwningGrid)))) _z) "0, 0, 0" false true (/ (* (Variables|Default|GetSteps) (Variables|/Script/Break2Bricks.Break2BricksBlockGrid|GetBlockSpacing (Variables|Default|GetOwningGrid))) (Variables|Default|GetDropDownSpeed)) false)
  (Variables|Default|SetbAnimConnectColumns false))

(fn ConstructionScript)